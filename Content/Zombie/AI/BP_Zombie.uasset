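; Zombie enemy that chases a player assigned by BP_GamePlayGM, attacks in melee and awards gold to its killer.
; AIMoveTo leads into a looping attack montage whose notify-driven sphere trace damages FPSCharacter, resuming pursuit when the target moves away.
; A timer reissues the chase whenever the zombie stands still.
; AnyDamage lowers CurHP, whose RepNotify updates an overhead health widget that a timer turns toward the local camera.
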(event Custom|ChasePlayer
  ;[1 1 1] 플레이어 쫓기
  (Utilities|IsValid (Variables|Default|GetChaseChar)
    (:Is%20Valid
      (AI|AIMoveTo self "0, 0, 0" (Variables|Default|GetChaseChar) 1.1e+02 false
        (:OnSuccess
          (CallFunction|Attack))))
    (:Is%20Not%20Valid
      (CallFunction|SetChar))))

(event Custom|Attack
  ;[1 1 1] 플레이어 공격
  (Utilities|IsValid (Variables|Default|GetChaseChar)
    (:Is%20Valid
      (Transformation|SetActorRotation (Math|Rotator|FindLookatRotation (Transformation|GetActorLocation self) (Transformation|GetActorLocation (Variables|Default|GetChaseChar))))
      (CallFunction|PlayAttackMontange))
    (:Is%20Not%20Valid
      (CallFunction|SetChar))))

(event Custom|AttackTrace
  (bind _returnvalue (Transformation|GetActorRotation))
  (bind _returnvalue_2 (Transformation|GetActorLocation))
  (bind _returnvalue_3 (Math|Vector|GetForwardVector _returnvalue))
  ;[1 1 1] AnimNotify로 불러올 함수내용
  (bind (_outhit _returnvalue_4) (Collision|SphereTraceForObjects (+ _returnvalue_2 (* _returnvalue_3 1e+02)) (+ _returnvalue_2 (* _returnvalue_3 1.7e+02)) 3e+01 (Utilities|Array|MakeArray "ObjectTypeQuery3") false 0 "None"))
  (if _returnvalue_4
    (bind _asfpscharacter (Utilities|Casting|CastToFPSCharacter (.HitActor (Collision|BreakHitResult _outhit))))
    (Class|FPSCharacter|GetDamage _asfpscharacter 1e+01)))

(event Custom|PlayAttackMontange
  ;[1 1 1] 적 공격 애니메이션
  (Animation|Montage|PlayMontage (Variables|Character|GetMesh) "/Game/Zombie/Animation/Zombie_Attack_Montage.Zombie_Attack_Montage" 3.0
    (:OnCompleted
      (Utilities|IsValid (Variables|Default|GetChaseChar)
        (:Is%20Valid
          (if (> (Math|Vector|Distance(Vector) (Transformation|GetActorLocation self) (Transformation|GetActorLocation (Variables|Default|GetChaseChar))) 1.5e+02)
            (CallFunction|ChasePlayer)
            (else
              (CallFunction|Attack))))
        (:Is%20Not%20Valid
          (CallFunction|SetChar))))))

(event Custom|GetGameMode
  ;[1 1 1] Comment
  (bind _asbp_game_play_gm (Utilities|Casting|CastToBP_GamePlayGM (Game|GetGameMode))
    (:then
      (Variables|Default|SetAs%20BP%20Game%20Play%20GM _asbp_game_play_gm))
    (:CastFailed
      (Utilities|Time|SetTimerbyFunctionName 0 "GetGameMode" 0.1))))

(event Custom|SetChar
  (bind _as_bp_game_play_gm (Variables|Default|GetAs%20BP%20Game%20Play%20GM))
  ;[1 1 1] 쫓을 플레이어 설정
  (Utilities|IsValid (Variables|Default|GetChaseChar)
    (:Is%20Not%20Valid
      (Utilities|IsValid _as_bp_game_play_gm
        (:Is%20Valid
          (Default|ResetChasePlayer _as_bp_game_play_gm self)
          (Utilities|IsValid (Variables|Default|GetChaseChar)
            (:Is%20Valid
              (CallFunction|ChasePlayer))
            (:Is%20Not%20Valid
              (CallFunction|SetChar))))))))

(event Custom|CheckCurPosition
  (bind _returnvalue (Transformation|GetActorLocation))
  ;[1 1 1] Comment
  (if (Utilities|Operators|EqualEqual (Variables|Default|GetCurlocation) _returnvalue 0.0)
    (CallFunction|ChasePlayer)
    (else
      (Variables|Default|SetCurlocation _returnvalue))))

(event EventBeginPlay
  ;[1 1 1] BeginPlay
  (CallFunction|GetGameMode)
  (Utilities|FlowControl|Delay 0.5)
  (CallFunction|ChasePlayer)
  (Variables|Default|SetCurHP (Variables|Default|GetMaxHP))
  (Utilities|Time|SetTimerbyFunctionName 0 "CheckCurPosition" 1.0 true)
  (Utilities|Time|SetTimerbyFunctionName 0 "HPLookAtPlayer" 0.2 true))

(event EventUpdateHP
  (params (Damage :type Float%20%28single-precision%29) (CurPlayer :type Player%20Controller%20Object%20Reference)))

(event Game|Damage|EventAnyDamage
  (params (Damage :type Float%20%28single-precision%29) (DamageType :type Damage%20Type%20Object%20Reference) (InstigatedBy :type Controller%20Object%20Reference) (DamageCauser :type Actor%20Object%20Reference))
  ;[1 1 1] GetDamage
  (bind _output_get (Variables|Default|SetCurHP (- (Variables|Default|GetCurHP) Damage)))
  (if (<= _output_get 0.0)
    (bind _asplayer_controller (Utilities|Casting|CastToPlayerController InstigatedBy)
      (:then
        (Default|UpdatePlayerGold (.AsBP%20Game%20Play%20GM (Utilities|Casting|CastToBP_GamePlayGM (Game|GetGameMode))) (Variables|Default|GetDropGold) _asplayer_controller)
        (Actor|DestroyActor))
      (:CastFailed
        (Development|PrintString "CantGetController")))))

(fn ConstructionScript)

(fn OnRepCurHP
  (bind _hpwidget (Variables|Default|GetHpWidget))
  (bind _returnvalue (UserInterface|GetWidget _hpwidget))
  (Utilities|IsValid _returnvalue
    (:Is%20Valid
      (bind _ashptag_widget (Utilities|Casting|CastToHPTagWidget _returnvalue))
      (Default|SetHp _ashptag_widget (/ (Variables|Default|GetCurHP) (Variables|Default|GetMaxHP))))
    (:Is%20Not%20Valid
      (Utilities|Time|SetTimerbyFunctionName 0 "OnRep_CurHP" 0.1))))

(fn SetWidgetRef
  (bind _hpwidget (Variables|Default|GetHpWidget))
  (bind _returnvalue (UserInterface|GetWidget _hpwidget))
  (Utilities|IsValid _returnvalue
    (:Is%20Valid
      (bind _ashptag_widget (Utilities|Casting|CastToHPTagWidget _returnvalue))
      (Variables|Default|SetHPTagWidgetRef _ashptag_widget))
    (:Is%20Not%20Valid
      (Utilities|Time|SetTimerbyFunctionName 0 "SetWidgetRef" 0.1))))

(fn HPLookatPlayer
  (Transformation|SetWorldRotation (Variables|Default|GetHpWidget) (Math|Rotator|FindLookatRotation (Transformation|GetWorldLocation (Variables|Default|GetHpWidget)) (Transformation|GetActorLocation (Game|GetPlayerCameraManager 0))) false false))