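; Game instance that handles multiplayer session hosting, joining and teardown for the lobby flow.
; LaunchLobby stores the host's settings, shows a loading screen, creates an Advanced Sessions session tagged with the server name, then opens Lobby as a listen server.
; Joining shows the loading screen and joins the given search result, while DestroySessionCall destroys the session.
; JoinServer is empty, and older create and join nodes remain disconnected.
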(event Custom|Joining
  (params (SearchResult :type Blueprint%20Session%20Result%20Structure%20%28by%20ref%29) (PlayerController :type Player%20Controller%20Object%20Reference))
  (Class|AllGameInstance|ShowLoadingScreen)
  (|JoinSession PlayerController SearchResult
    (:then
      (Input|SetInputModeGameOnly (Game|GetPlayerController 0) false))))

(event EventLaunchLobby
  (params (NumberOfPlayers :type Integer) (EnableLan :type Boolean) (ServerName :type Text%20%28by%20ref%29))
  (bind _returnvalue (Game|GetPlayerController 0))
  ;[1 1 1] CreateSession By AdvancedSession -> Host Menu에서 Create버튼 클릭시
  (Variables|Default|SetMaxPlayers NumberOfPlayers)
  (Variables|Default|SetLobbyName ServerName)
  (Class|AllGameInstance|ShowLoadingScreen)
  (|AdvancedSession (Utilities|Array|MakeArray (Class|AdvancedSessionsLibrary|MakeLiteralSessionPropertyString "ServerName" (Utilities|String|ToString(Text) ServerName)) "") _returnvalue (Variables|Default|GetMaxPlayers) 0 EnableLan true false true true true false false false true false true
    (:OnSuccess
      (Game|OpenLevel(byName) "Lobby" true "listen")
      (Input|SetInputModeGameOnly _returnvalue false))
    (:OnFailure
      (Development|PrintString "Failed to Create Session, TryAgain" true true "(R=0.000000,G=0.660000,B=1.000000,A=1.000000)" 1e+01))))

(event EventJoinServer
  (params (SessionToJoin :type Blueprint%20Session%20Result%20Structure))
  ;[1 1 1] Join Session -> Join Button 클릭 시
)

(event EventDestroySessionCall
  (params (PlayerController :type Player%20Controller%20Object%20Reference))
  ;[1 1 1] DestroySession
  (|DestroySession PlayerController))