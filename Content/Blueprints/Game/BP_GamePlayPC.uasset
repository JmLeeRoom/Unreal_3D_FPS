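; BP_GamePlayPC is the gameplay player controller that gets each player's saved character choice spawned through BP_GamePlayGM.
; On BeginPlay, the local controller clears widgets, sets game-only input and loads PlayerSettings from the save slot.
; It passes those settings to the server-side controller, which asks the game mode to respawn the chosen character.
; On EndPlay it reports itself to the game mode through DeadPlayer.
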(event Custom|PassCharaceterInfoToServer
  (params (PlayerSettingsInfo :type Player%20Info%20Structure))
  (Variables|Default|SetPlayerSettings PlayerSettingsInfo)
  (bind _asbp_game_play_gm (Utilities|Casting|CastToBP_GamePlayGM (Game|GetGameMode)))
  (Default|RespawnPlayer _asbp_game_play_gm self (.MyPlayerCharacter (Utilities|Struct|BreakPlayerInfo (Variables|Default|GetPlayerSettings)))))

(event EventEndPlay
  (params (EndPlayReason :type EEndPlayReason%20Enum :default "Destroyed"))
  (bind _asbp_game_play_gm (Utilities|Casting|CastToBP_GamePlayGM (Game|GetGameMode))
    (:then
      (Default|DeadPlayer _asbp_game_play_gm self))
    (:CastFailed
      (Development|PrintString "NoGMInPC"))))

(event EventBeginPlay
  ;[1 1 1] LoadPlayer Info and Pass to Serverside Player Controller
  (if (Pawn|IsLocalController)
    (Viewport|RemoveAllWidgets)
    (CallFunction|LoadGame)
    (Input|SetInputModeGameOnly self false)
    (CallFunction|PassCharaceterInfotoServer (Variables|Default|GetPlayerSettings))))

(fn ConstructionScript)

(fn LoadGame
  (bind _returnvalue (SaveGame|LoadGamefromSlot (Variables|Default|GetPlayerSettingsSave)))
  (bind _asplayer_save_game (Utilities|Casting|CastToPlayerSaveGame _returnvalue))
  (Variables|Default|SetPlayerSettings (Variables|/Script/Title2Lobby.PlayerSaveGame|GetS_PlayerInfo _asplayer_save_game)))